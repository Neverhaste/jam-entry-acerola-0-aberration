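; Behavior tree task that sends an AI agent to the location in a blackboard key and detects when it gets stuck.
; Execute starts the move; each tick treats Idle status as success, while other statuses time how long horizontal speed stays under a threshold, failing on timeout.
; Both outcomes clear the destination key and stop movement.
; Abort only stops movement, leaving the key and stuck timer untouched.
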(event Custom|Clear%20Navigation
  (params (bSuccess :type Boolean))
  (AI|BehaviorTree|FinishExecute bSuccess)
  (Class|BTFunctionLibrary|ClearBlackboardValue (Variables|Settings|GetDestination%20Key))
  (Utilities|IsValid (stale EventReceiveTickAI OwnerController)
    (:Is%20Valid
      (AI|Navigation|StopMovement (stale EventReceiveTickAI OwnerController))
      (Variables|Default|Set_stuckStartSeconds 0.0))))

(event EventReceiveExecuteAI
  (params (OwnerController :type AI%20Controller%20Object%20Reference) (ControlledPawn :type Pawn%20Object%20Reference))
  (Variables|Default|Set_stuckSpeedSquared (Math|Float|Square (Variables|Settings|GetStuck%20Speed%20Threshold)))
  (AI|Navigation|MovetoLocation OwnerController (Class|BTFunctionLibrary|GetBlackboardValueasVector (Variables|Settings|GetDestination%20Key)) 1.0 true true true false "/Script/AIModule.NavFilter_AIControllerDefault" false))

(event EventReceiveAbortAI
  (params (OwnerController :type AI%20Controller%20Object%20Reference) (ControlledPawn :type Pawn%20Object%20Reference))
  (AI|Navigation|StopMovement OwnerController)
  (Class|BTTaskBlueprintBase|FinishAbort))

(event EventReceiveTickAI
  (params (OwnerController :type AI%20Controller%20Object%20Reference) (ControlledPawn :type Pawn%20Object%20Reference) (DeltaSeconds :type Float%20%28single-precision%29))
  (switch Utilities|FlowControl|Switch|SwitchonEPathFollowingStatus (Class|AIController|GetMoveStatus OwnerController)
    (:Idle
      ;[0.4826 1 0.4984] Success
      (CallFunction|ClearNavigation true))
    (:Waiting
      (Utilities|FlowControl|Sequence :!label _label
        (:then_1
          ;[1 0.4906 0] Stuck Handling
          (if (<= (Class|KismetMathLibrary|VSizeXYSquared (Transformation|GetVelocity ControlledPawn)) (Variables|Default|Get_stuckSpeedSquared)) :!label _label_2
            (if (<= (Variables|Default|Get_stuckStartSeconds) 0.0)
              (Variables|Default|Set_stuckStartSeconds (Utilities|Time|GetGameTimeinSeconds))
              (elif (and (>= (- (Utilities|Time|GetGameTimeinSeconds) (Variables|Default|Get_stuckStartSeconds)) (Variables|Settings|GetStuck%20Timeout)) (!= 0.0 (Variables|Default|Get_stuckStartSeconds)))
                (CallFunction|ClearNavigation false)))
            (else
              (Variables|Default|Set_stuckStartSeconds 0.0))))))
    (:Paused
      (goto _label))
    (:Moving
      (goto _label_2))))