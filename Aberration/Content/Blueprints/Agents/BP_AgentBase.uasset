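; BP_AgentBase is a base agent Blueprint that can be selected and sent to a navigation target.
; On BeginPlay it caches its AI controller as a BP_AgentController.
; Selection events from BP_SelectableComponent show or hide a selection marker decal.
; SetNavigationTarget forwards a location to the cached controller's NavigateTo.
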(event OnSelected(BP_SelectableComponent)
  (Rendering|SetVisibility (Variables|Default|GetSelection%20Marker%20Decal) true false))

(event OnDeselected(BP_SelectableComponent)
  (Rendering|SetVisibility (Variables|Default|GetSelection%20Marker%20Decal) false false))

(event EventBeginPlay
  (bind _asbp_agent_controller (Utilities|Casting|CastToBP_AgentController (AI|GetAIController self)))
  (Variables|Default|SetAIController _asbp_agent_controller))

(fn ConstructionScript)

(fn SetNavigationTarget
  (params (Location :type Vector))
  (Default|Navigateto (Variables|Default|GetAIController) Location))