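; BP_SelectableComponent is a component that tracks whether it is selected and which selection holds it.
; Select removes it from any previous selection before adding it to the given one, so it follows one current selection at a time.
; Deselect acts only when the given selection matches the current one, and Toggle switches between the two.
; Both state changes call selected or deselected notifications.
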(fn GetIsSelected
  (return (Variables|Default|GetIs%20Selected)))

(fn Select
  (params (Selection :type BP%20Selection%20Object%20Reference))
  (if (Variables|Default|GetIs%20Selected)
    (Default|Remove (Variables|Default|GetCurrent%20Selection) self))
  (bind _output_get (Variables|Default|SetCurrent%20Selection Selection))
  (Default|Add _output_get self)
  (Variables|Default|SetIs%20Selected true)
  (Default|CallOnSelected))

(fn Deselect
  (params (Selection :type BP%20Selection%20Object%20Reference))
  (if (and (Variables|Default|GetIs%20Selected) (== Selection (Variables|Default|GetCurrent%20Selection)))
    (Default|Remove (Variables|Default|GetCurrent%20Selection) self)
    (Variables|Default|SetIs%20Selected false)
    (Default|CallOnDeselected)))

(fn Toggle
  (params (Selection :type BP%20Selection%20Object%20Reference))
  (if (Variables|Default|GetIs%20Selected)
    (CallFunction|Deselect Selection)
    (else
      (CallFunction|Select Selection))))