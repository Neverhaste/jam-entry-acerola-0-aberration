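; BP_Selection holds the list of currently selected objects.
; Add and Remove edit the list directly, without calling into the selectable.
; Clear repeatedly calls Deselect on the first entry, passing itself, until the list is empty, so it relies on each selectable removing itself from the list.
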(fn Add
  (params (Selectable :type BP%20Selectable%20Component%20Object%20Reference))
  (Utilities|Array|Add (Variables|Default|GetList) Selectable))

(fn Remove
  (params (Selectable :type BP%20Selectable%20Component%20Object%20Reference))
  (Utilities|Array|RemoveItem (Variables|Default|GetList) Selectable))

(fn Clear
  (bind _list (Variables|Default|GetList))
  (while (!= (Utilities|Array|Length _list) 0)
    (Default|Deselect (Utilities|Array|Get(acopy) _list) self)))