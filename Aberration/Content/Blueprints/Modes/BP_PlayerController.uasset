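; Player controller for a top-down command mode that drives a BP_TopDownCamera pawn and selects and orders agents.
; Tick feeds WASD pan, right-drag orbit (cursor pinned to its press point) and axis-driven distance into the camera.
; Left click replaces the BP_Selection, while dragging brush-adds selectable components under the cursor.
; An unmoved right click off any selectable sends selected agents to the WorldStatic hit point.
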(event EventBeginPlay
  (bind _asbp_top_down_camera (Utilities|Casting|CastToBP_TopDownCamera (Pawn|GetControlledPawn)))
  (Variables|Default|SetPlayer%20Pawn _asbp_top_down_camera)
  (Variables|Default|SetbShowMouseCursor true)
  (bind _returnvalue (Game|ConstructObjectfromClass "/Game/Blueprints/Selection/BP_Selection.BP_Selection_C" self))
  (Variables|Default|SetCommand%20Selection _returnvalue))

(event EventTick
  (params (DeltaSeconds :type Float%20%28single-precision%29))
  (bind (_deltax _deltay) (Class|PlayerController|GetInputMouseDelta))
  (bind _mouse_position_offset (Variables|Default|GetMouse%20Position%20Offset))
  (bind _player_pawn (Variables|Default|GetPlayer%20Pawn))
  (Utilities|FlowControl|Sequence
    (:then_0
      (if (Variables|Default|GetIs%20Orbitting)
        (Variables|Default|SetOrbit%20Vector (Math|Vector|MakeVector 0.0 _deltay _deltax))
        (Class|PlayerController|SetMouseLocation (.x _mouse_position_offset) (.y _mouse_position_offset))
        (else
          (Variables|Default|SetOrbit%20Vector (Math|Vector|MakeVector 0.0 0.0 0.0))))
      (Variables|Default|SetDistance (Class|Actor|GetInputAxisKeyValue)))
    (:then_1
      (Variables|Default|SetPan%20Vector (Math|Vector|MakeVector (- (Math|Conversions|ToFloat(Boolean) (Game|Player|IsInputKeyDown "W")) (Math|Conversions|ToFloat(Boolean) (Game|Player|IsInputKeyDown "S"))) (- (Math|Conversions|ToFloat(Boolean) (Game|Player|IsInputKeyDown "D")) (Math|Conversions|ToFloat(Boolean) (Game|Player|IsInputKeyDown "A"))) 0.0)))
    (:then_2
      (Default|AddPanInput _player_pawn (Math|Transform|TransformDirection (Default|GetDirectionalTransform _player_pawn) (Variables|Default|GetPan%20Vector)))
      (Default|AddOrbitInput _player_pawn (Variables|Default|GetOrbit%20Vector))
      (Default|AddDistanceInput _player_pawn (Variables|Default|GetDistance)))
    (:then_3
      (if (Variables|Default|GetIs%20Selecting)
        (if (CallFunction|HasMouseMovedfromOffset)
          (Variables|Default|SetIs%20Brush%20Selecting true))))
    (:then_4
      (if (Variables|Default|GetIs%20Brush%20Selecting)
        (bind _returnvalue (Utilities|GetSelectableUnderCursor)
          (:then
            (Default|Select _returnvalue (Variables|Default|GetCommand%20Selection))))))))

(event Input|KeyboardEvents|W
  (params (Key :type Key%20Structure :default "None")))

(event Input|KeyboardEvents|S
  (params (Key :type Key%20Structure :default "None")))

(event Input|KeyboardEvents|A
  (params (Key :type Key%20Structure :default "None")))

(event Input|KeyboardEvents|D
  (params (Key :type Key%20Structure :default "None")))

(event Input|MouseEvents|RightMouseButton
  (params (Key :type Key%20Structure :default "None"))
  (bind (_locationx _locationy) (Game|Player|GetMousePosition))
  (bind _array (Utilities|Array|MakeArray "ObjectTypeQuery1"))
  (bind (_hitresult _returnvalue) (Class|PlayerController|GetHitResultUnderCursorforObjects _array true))
  (:Pressed
    (Variables|Default|SetIs%20Orbitting true)
    (Variables|Default|SetbShowMouseCursor false)
    (Variables|Default|SetMouse%20Position%20Offset (Utilities|Struct|MakeIntVector (Math|Float|Truncate _locationx) (Math|Float|Truncate _locationy) 0)))
  (:Released
    (Variables|Default|SetIs%20Orbitting false)
    (Variables|Default|SetbShowMouseCursor true)
    (if (not (CallFunction|HasMouseMovedfromOffset))
      (Utilities|GetSelectableUnderCursor
        (:Fail
          (if _returnvalue
            (for _array_element (Default|GetAllAgents (Variables|Default|GetCommand%20Selection))
              (Default|SetNavigationTarget _array_element (.ImpactPoint (Collision|BreakHitResult _hitresult))))))))))

(event Input|MouseEvents|LeftMouseButton
  (params (Key :type Key%20Structure :default "None"))
  (bind (_locationx _locationy) (Game|Player|GetMousePosition))
  (:Pressed
    (Variables|Default|SetIs%20Selecting true)
    (Variables|Default|SetMouse%20Position%20Offset (Utilities|Struct|MakeIntVector (Math|Float|Truncate _locationx) (Math|Float|Truncate _locationy) 0)))
  (:Released
    (Variables|Default|SetIs%20Selecting false)
    (if (Variables|Default|GetIs%20Brush%20Selecting)
      (Variables|Default|SetIs%20Brush%20Selecting false)
      (else
        (Default|Clear (Variables|Default|GetCommand%20Selection))
        (bind _returnvalue (Utilities|GetSelectableUnderCursor)
          (:then
            (Default|Select _returnvalue (Variables|Default|GetCommand%20Selection))))))))

(fn ConstructionScript)

(fn HasMouseMovedfromOffset
  (bind (_locationx _locationy) (Game|Player|GetMousePosition))
  (bind _mouse_position_offset (Variables|Default|GetMouse%20Position%20Offset))
  (return (or (!= (.x _mouse_position_offset) (Math|Float|Truncate _locationx)) (!= (.y _mouse_position_offset) (Math|Float|Truncate _locationy)))))